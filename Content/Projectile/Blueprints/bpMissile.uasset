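; Missile projectile Blueprint that aligns its mesh and blast components to the mesh's Pivot socket at construction.
; The construction script calls FixLocation, which offsets the actor's location by the difference between the mesh's relative location and the Pivot socket location.
; It then re-attaches the LaunchBlast and ImpactBlast components to that socket, keeping relative transforms.
; The event graph holds no active logic.
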(event EventBeginPlay)

(event Collision|EventActorBeginOverlap
  (params (OtherActor :type Actor%20Object%20Reference)))

(event EventTick
  (params (DeltaSeconds :type Float%20%28single-precision%29)))

(fn ConstructionScript
  (MissileUtilities|FixLocation))

(fn FixLocation
  (bind _mesh (Variables|Character|GetMesh))
  (Utilities|FlowControl|Sequence
    (:then_0
      ;[1 1 1] Set correct position of the mesh using Pivot Socket
      (Transformation|SetActorLocation (+ (Transformation|GetActorLocation) (- (Variables|/Script/Engine.SceneComponent|GetRelativeLocation _mesh) (Transformation|GetSocketLocation _mesh "Pivot"))) false false))
    (:then_1
      ;[1 1 1] Re-attach Launch Blast to Mesh properly on Pivot Socket
      (Transformation|AttachComponentToComponent (Variables|Default|GetLaunchBlast) (Variables|Character|GetMesh) "Pivot" "KeepRelative" "KeepRelative" "KeepRelative" true))
    (:then_2
      ;[1 1 1] Re-attach Impact Blast to Mesh properly on Pivot socket
      (Transformation|AttachComponentToComponent (Variables|Default|GetImpactBlast) (Variables|Character|GetMesh) "Pivot" "KeepRelative" "KeepRelative" "KeepRelative" true))))