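; Player-controllable tank that acts as a hub, delegating driving to a Movement component and turret aiming and firing to an Aiming component.
; BeginPlay hands the turret, muzzle and tracks to those components and sets the tank as owner of its HealthUI widget.
; Aim axes orbit the camera at a frame-rate-independent speed, splitting yaw onto a Gimbal and pitch onto the SpringArm.
; Tick draws a red debug line forward from the muzzle.
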(event EventBeginPlay
  (Utilities|FlowControl|Sequence
    (:then_0
      ;[1 1 1] Initialise Turret for aiming
      (Class|AimingComponent|Initialise (Variables|Default|GetAiming) (Variables|Default|GetTurret) (Variables|Default|GetMuzzle)))
    (:then_1
      ;[1 1 1] Initialise Tracks for movement
      (Class|TankMovementComponent|Initialise (Variables|Default|GetMovement) (Variables|Default|GetLeftTrack) (Variables|Default|GetRightTrack)))
    (:then_2
      (CallFunction|InitialiseHealthBar))))

(event EventTick
  (params (DeltaSeconds :type Float%20%28single-precision%29))
  (CallFunction|DrawDebugLine))

(event Input|ActionEvents|InputActionFire
  (params (Key :type Key%20Structure :default "AnyKey"))
  ;[1 1 1] Action
  (:Pressed
    (Class|AimingComponent|Fire (Variables|Default|GetAiming))))

(event Input|AxisEvents|InputAxisTurn
  (params (AxisValue :type Float%20%28single-precision%29))
  ;[1 1 1] Movement
  (Class|TankMovementComponent|Turn (Variables|Default|GetMovement) AxisValue))

(event Input|AxisEvents|InputAxisAimAzimuth
  (params (AxisValue :type Float%20%28single-precision%29))
  ;[1 1 1] Camera rotation
  (CallFunction|RotateArm AxisValue false))

(event Input|AxisEvents|InputAxisAimElevation
  (params (AxisValue :type Float%20%28single-precision%29))
  ;[1 1 1] Camera rotation
  (CallFunction|RotateArm AxisValue true))

(event Input|AxisEvents|InputAxisMove
  (params (AxisValue :type Float%20%28single-precision%29))
  ;[1 1 1] Movement
  (Class|TankMovementComponent|Move (Variables|Default|GetMovement) AxisValue))

(fn ConstructionScript)

(fn RotateArm
  (params (Angle :type Float%20%28single-precision%29) (Pitch%20%28T%29%20|%20Yaw%20%28F%29 :type Boolean))
  (Utilities|FlowControl|Sequence
    (:then_0
      (LocalVariables|SetDeltaRotation (* Angle (Utilities|Time|GetWorldDeltaSeconds) 1e+02)))
    (:then_1
      (if Pitch%20%28T%29%20|%20Yaw%20%28F%29
        (LocalVariables|SetDeltaPitch (LocalVariables|GetDeltaRotation))
        (LocalVariables|SetComponentToRotate (Variables|Default|GetSpringArm))
        (else
          (LocalVariables|SetDeltaYaw (LocalVariables|GetDeltaRotation))
          (LocalVariables|SetComponentToRotate (Variables|Default|GetGimbal)))))
    (:then_2
      (Transformation|AddLocalRotation (LocalVariables|GetComponentToRotate) (Math|Rotator|MakeRotator 0.0 (LocalVariables|GetDeltaPitch) (LocalVariables|GetDeltaYaw)) false false))))

(fn DrawDebugLine
  (bind _muzzle (Variables|Default|GetMuzzle))
  (bind _returnvalue (Transformation|GetWorldLocation _muzzle))
  (Rendering|Debug|DrawDebugLine _returnvalue (+ _returnvalue (* (Math|Vector|GetForwardVector _muzzle) 500)) "(R=1.000000,G=0.000000,B=0.000000,A=1.000000)" 0.01 5.0))

(fn InitialiseHealthBar
  (bind _ashealth_ui (Utilities|Casting|CastToHealthUI (UserInterface|GetUserWidgetObject (Variables|Default|GetHealthBar))))
  (Variables|/Game/UI/Blueprints/HealthUI.HealthUI_C|SetOwner _ashealth_ui self))